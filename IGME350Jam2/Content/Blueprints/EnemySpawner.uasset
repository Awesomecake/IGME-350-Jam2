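; Enemy spawner that continuously creates EnemyBP actors around a set of spawn points, starting at BeginPlay.
; A looping half-second delay picks a random spawn point and spawns at a random navigable location close to it.
; Each valid enemy gets a GoalPosition from the spawn point after a randomly drawn index, wrapping around the array.
; That second draw is re-evaluated, so the goal is not tied to the origin point.
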(event EventBeginPlay
  (bind _spawnpoints (Variables|Default|GetSpawnPoints))
  (bind (_outitem _outindex) (Utilities|Array|Random _spawnpoints))
  (Utilities|FlowControl|Delay 0.5 :!label _label)
  (bind _randomlocation (Class|NavigationSystemV1|GetRandomLocationinNavigableRadius (Transformation|GetActorLocation _outitem) 1e+01 0 0))
  (bind _returnvalue (Game|SpawnActorfromClass "/Game/Blueprints/EnemyBP.EnemyBP_C" (Math|Conversions|ToTransform(Vector) _randomlocation) "Undefined" "MultiplyWithRoot" 0 0))
  (Utilities|IsValid _returnvalue
    (:Is%20Valid
      (Variables|/Game/Blueprints/EnemyBP.EnemyBP_C|SetGoalPosition _returnvalue (Transformation|GetActorLocation (Utilities|Array|Get(acopy) (Variables|Default|GetSpawnPoints) (Math|Integer|%(Integer) (+ _outindex 1) (Utilities|Array|Length _spawnpoints)))))
      (goto _label))
    (:Is%20Not%20Valid
      (goto _label))))

(fn ConstructionScript)
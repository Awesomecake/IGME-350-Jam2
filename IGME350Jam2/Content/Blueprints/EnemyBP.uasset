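; EnemyBP is a short-lived shooting target that walks toward GoalPosition via AIMoveTo, reissued every Tick.
; BeginPlay randomly flags it as a customer, swapping to the farmer material, and destroys it after a few seconds.
; A projectile hit destroys both actors, spawns a ScoreVisual and updates the player's points: a penalty for customers, a reward otherwise.
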(event EventBeginPlay
  (Utilities|FlowControl|Sequence
    (:then_0
      (Utilities|FlowControl|Delay 4.0)
      (Actor|DestroyActor))
    (:then_1
      (bind _output_get (Variables|Default|SetIsCustomer (Math|Random|RandomBool)))
      (if _output_get
        (Rendering|Material|SetMaterial (Variables|Character|GetMesh) 0 "/Game/Animated_Characters_Bundle/Skins/farmerA_Mat.farmerA_Mat")))))

(event Collision|EventActorBeginOverlap
  (params (OtherActor :type Actor%20Object%20Reference)))

(event Collision|EventHit
  (params (MyComp :type Primitive%20Component%20Object%20Reference) (Other :type Actor%20Object%20Reference) (OtherComp :type Primitive%20Component%20Object%20Reference) (bSelfMoved :type Boolean) (HitLocation :type Vector :default "0, 0, 0") (HitNormal :type Vector :default "0, 0, 0") (NormalImpulse :type Vector :default "0, 0, 0") (Hit :type Hit%20Result%20Structure%20%28by%20ref%29))
  (bind _asbp_first_person_projectile (Utilities|Casting|CastToBP_FirstPersonProjectile Other))
  (Actor|DestroyActor _asbp_first_person_projectile)
  (bind _asbp_first_person_character (Utilities|Casting|CastToBP_FirstPersonCharacter (Pawn|GetControlledPawn (Game|GetPlayerController 0))))
  (bind _returnvalue (Game|SpawnActorfromClass "/Game/Blueprints/ScoreVisual.ScoreVisual_C" (Transformation|GetActorTransform) "AlwaysSpawn" "MultiplyWithRoot" 0 0))
  (if (Variables|Default|GetIsCustomer)
    (Default|UpdatePoints _asbp_first_person_character -100)
    (Default|ShowNegative _returnvalue)
    (else
      (Default|UpdatePoints _asbp_first_person_character 100)))
  (Actor|DestroyActor))

(event EventTick
  (params (DeltaSeconds :type Float%20%28single-precision%29))
  (AI|AIMoveTo self (Variables|Default|GetGoalPosition) 0 5.0 false))

(fn ConstructionScript)